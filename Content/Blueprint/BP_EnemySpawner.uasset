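; BP_EnemySpawner is a spawner actor that periodically creates enemies at its Arrow component's transform.
; Tick accumulates delta time, spawns an actor of SpawnClass once DelayTime is reached, then resets the timer.
; A disconnected random check against TraceRate is present but never runs.
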(event `self.ReceiveTick`
  (params (DeltaSeconds :type "Float (single-precision)"))
  (bind _output_get (set `self.CurrentTime` (+ DeltaSeconds (`self.CurrentTime`))))
  (if (>= _output_get (`self.DelayTime`))
    (`|SpawnActorFromClass` (`self.SpawnClass`) (`SceneComponent.K2_GetComponentToWorld` (`self.Arrow`)) "Undefined" "MultiplyWithRoot" null null)
    (set `self.CurrentTime` 0.0)))

(fn `UserConstructionScript`)
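; BP_Turret is a turret that periodically turns toward the first player's pawn and fires.
; Tick accumulates delta time in CheckCanAttack; once DelayTime is reached, it resets the timer, starts aiming and immediately spawns BulletClass at FirePositionArrow.
; The RotMove timeline lerps SubMesh's yaw using a rotation built from the target offset, then resets its time after a short delay.
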(event `self.ReceiveTick`
  (params (DeltaSeconds :type "Float (single-precision)"))
  (bind _done (`self.CheckCanAttack`))
  (if _done
    (`self.LerpTargetAim` (`GameplayStatics.GetPlayerPawn` 0))
    (`self.Fire` (`self.Bullet Class`))))

(event `LerpTargetAim`
  (params (`Target Actor` :type "Actor Object Reference"))
  (bind (_direction _lerpalpha) (`Timeline|RotMove` :!label _label)
    (:`Update`
      (`self.AimTarget` `Target Actor` _lerpalpha))
    (:`Finished`
      (`KismetSystemLibrary.Delay` 0.2)
      (goto _label :!via `SetNewTime`))))

(fn `AimTarget`
  (params (`Target Actor` :type "Actor Object Reference") (`Lerp Alpha` :type "Float (double-precision)"))
  (bind _submesh (`self.SubMesh`))
  (bind (_returnvalue_roll _returnvalue_pitch _returnvalue_yaw) (`KismetMathLibrary.BreakRotator` (`SceneComponent.K2_GetComponentRotation` _submesh)))
  (bind (_returnvalue_roll_2 _returnvalue_pitch_2 _returnvalue_yaw_2) (`KismetMathLibrary.BreakRotator` (`KismetMathLibrary.MakeRotFromZ` (`KismetMathLibrary.Normal` (- (`SceneComponent.K2_GetComponentLocation` _submesh) (`self.K2_GetActorLocation` `Target Actor`))))))
  (`/Engine/EditorBlueprintResources/StandardMacros.IsValid` `Target Actor`
    (:`Is Valid`
      (`SceneComponent.K2_SetWorldRotation` _submesh (`KismetMathLibrary.MakeRotator` 0.0 0.0 (`KismetMathLibrary.Lerp` _returnvalue_yaw _returnvalue_yaw_2 `Lerp Alpha`)) false false))))

(fn `CheckCanAttack`
  (returns (Done :type Boolean))
  (if (< (`self.TimerCurrentTime`) (`self.DelayTime`))
    (set `self.TimerCurrentTime` (+ (`GameplayStatics.GetWorldDeltaSeconds`) (`self.TimerCurrentTime`)))
    (return false)
    (else
      (set `self.TimerCurrentTime` 0.0)
      (return true))))

(fn `Fire`
  (params (BulletClass :type "Actor Class Reference"))
  (`|SpawnActorFromClass` BulletClass (`SceneComponent.K2_GetComponentToWorld` (`self.FirePositionArrow`)) "Undefined" "MultiplyWithRoot" null null))

(fn `UserConstructionScript`)
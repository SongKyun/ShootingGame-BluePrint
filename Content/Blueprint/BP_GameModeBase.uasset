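; Game mode for a tank game that picks the player's tank, tracks score and high score, and handles game over.
; The construction script sets the default pawn class from the selected index in GI_TankGame.
; BeginPlay loads the saved high score and shows the main UI; AddScore saves any new high score to a save slot.
; GameOver shows the game-over widget and mouse cursor, then pauses the game.
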(event `self.ReceiveBeginPlay`
  (`WidgetBlueprintLibrary.SetInputMode_GameOnly` (`GameplayStatics.GetPlayerController` 0))
  ;[1 1 1] 시작 시 0점 명시적 구현
  (set `self.Score` 0)
  (bind _highscore (`self.LoadScoreData`))
  (set `self.High Score` _highscore)
  (bind _returnvalue (`|CreateWidget` "/Game/UI/WBP_MainUI.WBP_MainUI_C"))
  (`UserWidget.AddToViewport` _returnvalue 0)
  (cast `/Game/Blueprint/GI_TankGame` (`GameplayStatics.GetGameInstance`)))

(fn `AddScore`
  (params (Increment :type Integer :default 2))
  ;[1 1 1] 점수 증가
  (bind _output_get (set `self.Score` (+ (`self.Score`) Increment)))
  (if (> _output_get (`self.High Score`))
    (bind _output_get_2 (set `self.High Score` _output_get))
    (`self.SaveScoreData` _output_get_2)))

(fn `ChangePlayerCharacter`
  (switch `int` (`/Game/Blueprint/GI_TankGame.SelectedIndex` (cast `/Game/Blueprint/GI_TankGame` (`GameplayStatics.GetGameInstance`) :!pure true))
    (:`Default`
      (set `self.DefaultPawnClass` "/Game/Blueprint/TankPlayer/BP_Player_Tank1.BP_Player_Tank1_C"))
    (:`0`
      (set `self.DefaultPawnClass` "/Game/Blueprint/TankPlayer/BP_Player_Tank1.BP_Player_Tank1_C"))
    (:`1`
      (set `self.DefaultPawnClass` "/Game/Blueprint/TankPlayer/BP_Player_Tank1_A.BP_Player_Tank1_A_C"))
    (:`2`
      (set `self.DefaultPawnClass` "/Game/Blueprint/TankPlayer/BP_Player_Tank1_B.BP_Player_Tank1_B_C"))
    (:`3`
      (set `self.DefaultPawnClass` "/Game/Blueprint/TankPlayer/BP_Player_Tank1_C.BP_Player_Tank1_C_C"))))

(fn `GameOver`
  (bind _returnvalue (`|CreateWidget` "/Game/UI/BP_GameOverUI.BP_GameOverUI_C"))
  (`UserWidget.AddToViewport` _returnvalue 0)
  (set `PlayerController.bShowMouseCursor` true (`GameplayStatics.GetPlayerController` 0))
  (`GameplayStatics.SetGamePaused` true))

(fn `LoadScoreData`
  (returns (HighScore :type Integer))
  (bind _slot_string (`self.Slot String`))
  (bind _returnvalue (`GameplayStatics.DoesSaveGameExist` _slot_string))
  (if _returnvalue
    (bind _returnvalue_2 (`GameplayStatics.LoadGameFromSlot` _slot_string))
    (bind _asbp_save_data (cast `/Game/Blueprint/BP_SaveData` _returnvalue_2))
    (return (`/Game/Blueprint/BP_SaveData.ScoreData` _asbp_save_data))))

(fn `SaveScoreData`
  (params (`Save Value` :type Integer))
  (bind _returnvalue (`GameplayStatics.CreateSaveGameObject` "/Game/Blueprint/BP_SaveData.BP_SaveData_C"))
  (bind _output_get (set `self.Save Instance` _returnvalue))
  (set `/Game/Blueprint/BP_SaveData.ScoreData` `Save Value` _output_get)
  (`GameplayStatics.SaveGameToSlot` _output_get (`self.Slot String`)))

(fn `UserConstructionScript`
  (`self.ChangePlayerCharacter`))
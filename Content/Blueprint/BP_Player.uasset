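; BP_Player is the player-controlled actor, which moves, turns, fires bullets and can be debuffed.
; Enhanced Input drives frame-time-scaled forward movement without sweep, per-event yaw rotation, and switching between two bullet classes.
; Firing spawns the selected bullet with a sound unless Disarm is active; Slow temporarily scales MoveSpeed, gated by CCState.
; Unconnected vector-math and timer test nodes remain in the event graph.
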(event `EnhancedInput|/Game/Preset/Input/IA/IA_Move`
  (params (ActionValue :type "Float (double-precision)") (ElapsedSeconds :type "Float (double-precision)") (TriggeredSeconds :type "Float (double-precision)") (InputAction :type "InputAction Object Reference" :default "/Game/Preset/Input/IA/IA_Move.IA_Move"))
  ;[1 1 1] 등속운동/현재 위치 + 이동거리
  (:`Triggered`
    (`self.MoveForward` ActionValue)))

(event `InputAction|Fire1`
  (params (Key :type "Key Structure"))
  ;[1 1 1] Fire
  (:`Pressed`
    (if (`self.IsCanAttack`)
      (`self.FireBulletActor`))))

(event `self.ReceiveBeginPlay`
  ;[1 1 1] IA 사용
  (bind _asplayer_controller (cast `PlayerController` (`self.GetController`)))
  (`EnhancedInputSubsystemInterface.AddMappingContext` (pcsubsystem `EnhancedInputLocalPlayerSubsystem` _asplayer_controller) "/Game/Preset/Input/IMC_Main.IMC_Main" 0 (struct)))

(event `EnhancedInput|/Game/Preset/Input/IA/IA_RotateBody`
  (params (ActionValue :type "Float (double-precision)") (ElapsedSeconds :type "Float (double-precision)") (TriggeredSeconds :type "Float (double-precision)") (InputAction :type "InputAction Object Reference" :default "/Game/Preset/Input/IA/IA_RotateBody.IA_RotateBody"))
  ;[1 1 1] 몸체 회전
  (:`Triggered`
    (`self.K2_AddActorWorldRotation` (`KismetMathLibrary.MakeRotator` 0.0 0.0 (* ActionValue (`self.Rotation Move Speed`))))))

(event `EnhancedInput|/Game/Preset/Input/IA/IA_Weapon`
  (params (ActionValue :type "Float (double-precision)") (ElapsedSeconds :type "Float (double-precision)") (TriggeredSeconds :type "Float (double-precision)") (InputAction :type "InputAction Object Reference" :default "/Game/Preset/Input/IA/IA_Weapon.IA_Weapon"))
  ;[1 1 1] 총알 스위칭
  (:`Started`
    (switch `int` (`KismetMathLibrary.FTrunc` ActionValue)
      (:`1`
        (set `self.Bullet Actor` "/Game/Blueprint/Bullet/BP_Bullet_Style1.BP_Bullet_Style1_C"))
      (:`2`
        (set `self.Bullet Actor` "/Game/Blueprint/Bullet/BP_Bullet_Style2.BP_Bullet_Style2_C")))))

(event `/Game/Blueprint/Interfaces/CrowControl.Disarm`
  (params (Duration :type "Float (double-precision)"))
  ;[1 1 1] 디버프
  (set `self.IsCanAttack` false)
  (`KismetSystemLibrary.Delay` Duration)
  (set `self.IsCanAttack` true))

(event `/Game/Blueprint/Interfaces/CrowControl.Slow`
  (params (Duration :type "Float (double-precision)") (`Slow Ratio` :type "Float (double-precision)"))
  ;[1 1 1] 디버프
  (if (not (`|EnumEquality` (`self.CCState`) "NewEnumerator1"))
    (set `self.MoveSpeed` (* `Slow Ratio` (`self.MoveSpeed`)))
    (set `self.CCState` "NewEnumerator0")
    (`KismetSystemLibrary.Delay` Duration)
    (set `self.MoveSpeed` (`self.InitMoveSpeed`))
    (set `self.CCState` "NewEnumerator0")))

(fn `FireBulletActor`
  (bind _fireposition_location (`KismetMathLibrary.BreakTransform` (`self.FirePosition`)))
  (`|SpawnActorFromClass` (`self.Bullet Actor`) (`self.FirePosition`) "Undefined" "MultiplyWithRoot" null null)
  (`GameplayStatics.PlaySoundAtLocation` "/Game/Interface_And_Item_Sounds/WAV/Abstract_Pop_01.Abstract_Pop_01" _fireposition_location (struct) 1.0 1.0 0.0 null null null null) ; 3D
)

(fn `MoveForward`
  (params (InputValue :type "Float (double-precision)"))
  (`self.K2_SetActorLocation` (+ (`self.K2_GetActorLocation`) (* InputValue (`self.MoveSpeed`) (`self.GetActorForwardVector`) (`GameplayStatics.GetWorldDeltaSeconds`)))))

(fn `UserConstructionScript`)
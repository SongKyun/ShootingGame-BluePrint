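; BP_Player_Tank1 is a player tank Blueprint that specializes its parent with a bullet type and head rotation.
; On BeginPlay it runs the parent logic, sets BP_Bullet_Style1 as the bullet and caches the fire arrow's world transform as FirePosition.
; The IA_RotateHead input refreshes FirePosition before yawing the static mesh, with each step clamped to RotationSpeed in either direction.
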(event `self.ReceiveBeginPlay`
  (`parent.ReceiveBeginPlay`)
  (set `self.Bullet Actor` "/Game/Blueprint/Bullet/BP_Bullet_Style1.BP_Bullet_Style1_C")
  (set `self.FirePosition` (`SceneComponent.K2_GetComponentToWorld` (`self.FirePositionArrow`))))

(event `EnhancedInput|/Game/Preset/Input/IA/IA_RotateHead`
  (params (ActionValue :type "Float (double-precision)") (ElapsedSeconds :type "Float (double-precision)") (TriggeredSeconds :type "Float (double-precision)") (InputAction :type "InputAction Object Reference" :default "/Game/Preset/Input/IA/IA_RotateHead.IA_RotateHead"))
  (bind _rotation_speed (`self.Rotation Speed`))
  (:`Triggered`
    (set `self.FirePosition` (`SceneComponent.K2_GetComponentToWorld` (`self.FirePositionArrow`)))
    (`SceneComponent.K2_AddLocalRotation` (`self.StaticMesh`) (`KismetMathLibrary.MakeRotator` 0.0 0.0 (`KismetMathLibrary.FClamp` ActionValue (* _rotation_speed -1.0) _rotation_speed)) false false)))

(fn `UserConstructionScript`
  (`parent.UserConstructionScript`))
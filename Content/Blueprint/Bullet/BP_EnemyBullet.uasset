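; BP_EnemyBullet is an enemy projectile that ends the game when it hits the player.
; Each Tick it moves along its forward vector at MoveSpeed by setting its location without sweep.
; A sphere overlap calls HitActor, which sends disarm and slow messages to the hit actor, then calls GameOver on BP_GameModeBase if that actor is the player pawn.
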(event `self.ReceiveTick`
  (params (DeltaSeconds :type "Float (single-precision)"))
  (`self.Move Foward` DeltaSeconds (`self.MoveSpeed`)))

(event `/Game/Blueprint/Interfaces/BulletActionInterface.Hit Actor`
  (params (`Target Actor` :type "Actor Object Reference") (Duration :type "Float (double-precision)") (`Slow Ratio` :type "Float (double-precision)"))
  (message `/Game/Blueprint/Interfaces/CrowControl.Disarm` `Target Actor` 0.0)
  (message `/Game/Blueprint/Interfaces/CrowControl.Slow` `Target Actor` 2.0 0.2)
  (if (== `Target Actor` (`GameplayStatics.GetPlayerPawn` 0))
    (`/Game/Blueprint/BP_GameModeBase.GameOver` (cast `/Game/Blueprint/BP_GameModeBase` (`GameplayStatics.GetGameMode`) :!pure true))))

(event `self.SphereBullet.OnComponentBeginOverlap`
  (params (OverlappedComponent :type "PrimitiveComponent Object Reference") (OtherActor :type "Actor Object Reference") (OtherComp :type "PrimitiveComponent Object Reference") (OtherBodyIndex :type Integer) (bFromSweep :type Boolean) (SweepResult :type "HitResult Structure (by ref)"))
  (`self.Hit Actor` OtherActor))

(fn `Move Foward`
  (params (`Delta Sec` :type "Float (double-precision)") (Speed :type "Float (double-precision)"))
  (`self.K2_SetActorLocation` (+ (`self.K2_GetActorLocation`) (* `Delta Sec` (* Speed (`self.GetActorForwardVector`))))))

(fn `UserConstructionScript`)
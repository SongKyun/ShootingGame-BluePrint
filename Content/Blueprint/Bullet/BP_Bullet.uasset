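; BP_Bullet is a projectile that moves along its forward vector each tick and hits actors it overlaps.
; Movement is a frame-rate-scaled location offset without sweep, and SphereCol overlaps call HitActor, defined outside this graph, with zero duration and slow ratio.
; BeginPlay caches BP_GameModeBase for DestroyTarget, which destroys an actor, adds score and plays effects.
; DestroyTarget's only call here, behind an enemy cast, is disconnected and never runs.
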(event `self.ReceiveActorBeginOverlap`
  (params (OtherActor :type "Actor Object Reference")))

(event `self.ReceiveBeginPlay`
  ;[1 1 1] 게임모드 캐싱(캐스트피하려고)
  (bind _asbp_game_mode_base (cast `/Game/Blueprint/BP_GameModeBase` (`GameplayStatics.GetGameMode`)))
  (set `self.As BP Game Mode Base` _asbp_game_mode_base))

(event `self.SphereCol.OnComponentBeginOverlap`
  (params (OverlappedComponent :type "PrimitiveComponent Object Reference") (OtherActor :type "Actor Object Reference") (OtherComp :type "PrimitiveComponent Object Reference") (OtherBodyIndex :type Integer) (bFromSweep :type Boolean) (SweepResult :type "HitResult Structure (by ref)"))
  (`self.Hit Actor` OtherActor))

(event `self.ReceiveTick`
  (params (DeltaSeconds :type "Float (single-precision)"))
  (`self.MoveForward`))

(fn `DestroyTarget`
  (params (`Target Actor` :type "Actor Object Reference") (`Destroy Effect` :type "ParticleSystem Object Reference") (`Destroy Sound` :type "SoundBase Object Reference") (`Score Point` :type Integer))
  (locals (ActorLocation :type "Vector Structure"))
  (bind _actorlocation (`local.ActorLocation`))
  (`/Engine/EditorBlueprintResources/StandardMacros.IsValid` `Target Actor`
    (:`Is Valid`
      (set `local.ActorLocation` (`self.K2_GetActorLocation` `Target Actor`))
      (`self.K2_DestroyActor` `Target Actor`)
      (`/Game/Blueprint/BP_GameModeBase.AddScore` (`self.As BP Game Mode Base`) `Score Point`)
      (`GameplayStatics.SpawnEmitterAtLocation` `Destroy Effect` _actorlocation)
      (`GameplayStatics.PlaySoundAtLocation` `Destroy Sound` _actorlocation (struct) 1.0 1.0 0.0 null null null null))))

(fn `MoveForward`
  (`self.K2_SetActorLocation` (+ (`self.K2_GetActorLocation`) (* (`self.GetActorForwardVector`) (`self.MoveSpeed`) (`GameplayStatics.GetWorldDeltaSeconds`)))))

(fn `UserConstructionScript`)
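; BP_Bullet_Style1 is a bullet Blueprint that damages enemies through a hit counter.
; On HitActor it acts only on BP_Enemy targets, destroying itself after each such hit.
; An enemy with HitCount at zero or below goes to DestroyTarget with explosion effect, pop sound and its ScorePoint.
; Otherwise the hit decrements HitCount, so the kill takes one hit beyond the count.
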(event `/Game/Blueprint/Interfaces/BulletActionInterface.Hit Actor`
  (params (`Target Actor` :type "Actor Object Reference") (Duration :type "Float (double-precision)") (`Slow Ratio` :type "Float (double-precision)"))
  (bind _asbp_enemy (cast `/Game/Blueprint/Enemy/BP_Enemy` `Target Actor`))
  (bind _hitcount (`/Game/Blueprint/Enemy/BP_Enemy.HitCount` _asbp_enemy))
  (if (<= _hitcount 0)
    (`self.DestroyTarget` _asbp_enemy "/Game/StarterContent/Particles/P_Explosion.P_Explosion" "/Game/Interface_And_Item_Sounds/WAV/Pop_06.Pop_06" (`/Game/Blueprint/Enemy/BP_Enemy.ScorePoint` _asbp_enemy))
    (`self.K2_DestroyActor`)
    (else
      (`/Engine/EditorBlueprintResources/StandardMacros.DecrementInt` _hitcount
        (:`  `
          (`self.K2_DestroyActor`))))))

(fn `UserConstructionScript`
  (`parent.UserConstructionScript`))
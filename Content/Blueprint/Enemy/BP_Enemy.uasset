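; BP_Enemy is an enemy actor with toggleable body-attack and ranged special-attack behaviors, both run from Tick.
; Body attack moves forward and re-aims at the player on a random TraceRate roll; special attack closes to FireDistance, then spawns bullets on a delay timer.
; Overlapping the player destroys it and spawns an emitter, while a box overlap calls BodyCheck.
; Slow temporarily scales move speed, then restores the initial value.
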(event `self.ReceiveTick`
  (params (DeltaSeconds :type "Float (single-precision)"))
  ;[1 1 1] Tick
  (`|ExecutionSequence`
    (:`then_0`
      (if (`self.bHasBodyAttack`)
        (`self.BodyAttack`)))
    (:`then_1`
      (if (`self.bHasSpecialAttack`)
        (bind _fire (`self.Move to Distance` (`GameplayStatics.GetPlayerPawn` 0)))
        (if _fire
          (bind _done (`self.Check Can Fire`))
          (if _done
            (`self.FireBullet` (`self.Bullet Class`))))))))

(event `self.ReceiveActorBeginOverlap`
  (params (OtherActor :type "Actor Object Reference"))
  ;[1 1 1] 적과 부딪힐 시 플레이어 삭제, GameOver
  (bind _asbp_player (cast `/Game/Blueprint/BP_Player` OtherActor))
  (`self.K2_DestroyActor` _asbp_player)
  (`GameplayStatics.SpawnEmitterAtLocation` null (`self.K2_GetActorLocation`)))

(event `self.BoxCol.OnComponentBeginOverlap`
  (params (OverlappedComponent :type "PrimitiveComponent Object Reference") (OtherActor :type "Actor Object Reference") (OtherComp :type "PrimitiveComponent Object Reference") (OtherBodyIndex :type Integer) (bFromSweep :type Boolean) (SweepResult :type "HitResult Structure (by ref)"))
  ;[1 1 1] 적과 부딪힐 시 플레이어 삭제, GameOver
  (if (== OtherActor (`GameplayStatics.GetPlayerPawn` 0))
    (`self.Body Check`)))

(event `/Game/Blueprint/Interfaces/CrowControl.Slow`
  (params (Duration :type "Float (double-precision)") (`Slow Ratio` :type "Float (double-precision)"))
  ;[1 1 1] slow
  (set `self.EMoveSpeed` (* `Slow Ratio` (`self.EMoveSpeed`)))
  (`KismetSystemLibrary.Delay` Duration)
  (set `self.EMoveSpeed` (`self.Init Move Speed`)))

(fn `BodyAttack`
  (`self.Move Foward Direction`)
  (if (<= (`KismetMathLibrary.RandomFloatInRange` 0.0 1.0) (`self.TraceRate`))
    (`self.Find Target Direction` (`GameplayStatics.GetPlayerPawn` 0))
    (else
      (set `self.Direction` (`self.GetActorForwardVector`)))))

(fn `Check Can Fire`
  (returns (Done :type Boolean))
  (if (< (`self.Timer Current Time`) (`self.Delay Time`))
    (set `self.Timer Current Time` (+ (`self.Timer Current Time`) (`GameplayStatics.GetWorldDeltaSeconds`)))
    (return false)
    (else
      (set `self.Timer Current Time` 0.0)
      (return true))))

(fn `Find Target Direction`
  (params (Target :type "Actor Object Reference"))
  (`/Engine/EditorBlueprintResources/StandardMacros.IsValid` Target
    (:`Is Valid`
      (set `self.Direction` (`KismetMathLibrary.Normal` (- (`self.K2_GetActorLocation` Target) (`self.K2_GetActorLocation`))))
      (`self.K2_SetActorRotation` (`KismetMathLibrary.FindLookAtRotation` (`self.K2_GetActorLocation`) (`self.K2_GetActorLocation` Target))))))

(fn `FireBullet`
  (params (`Bullet Class` :type "Actor Class Reference"))
  (`|SpawnActorFromClass` `Bullet Class` (`self.GetTransform`) "Undefined" "MultiplyWithRoot" null null))

(fn `Move Foward Direction`
  (`self.K2_SetActorLocation` (+ (`self.K2_GetActorLocation`) (* (`self.Direction`) (`self.EMoveSpeed`) (`GameplayStatics.GetWorldDeltaSeconds`)))))

(fn `Move to Distance`
  (params (`Target Actor` :type "Actor Object Reference"))
  (returns (Fire :type Boolean))
  (if (<= (`self.GetDistanceTo` `Target Actor`) (`self.Fire Distance`))
    (return true)
    (else
      (`self.Find Target Direction` `Target Actor`)
      (`self.Move Foward Direction`)
      (return false))))

(fn `UserConstructionScript`)
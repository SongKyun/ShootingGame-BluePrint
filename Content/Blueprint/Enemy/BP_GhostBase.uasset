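; Base Blueprint for ghost enemies that loads each ghost's stats from the DT_Ghost data table.
; The Construction Script passes RowIndex to Data Setup, which picks the row name at that index and copies movement, hit count, attack flags, score and fire-attack timing into variables.
; Rows are selected by position rather than by name, so table order determines each ghost's stats.
; The Event Graph holds no active logic.
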(fn `Data Setup`
  (params (`Row Index` :type Integer))
  (bind _outrownames (`DataTableFunctionLibrary.GetDataTableRowNames` "/Game/Blueprint/Enemy/DT_Ghost.DT_Ghost"))
  (bind _returnvalue (`|GetDataTableRow` "/Game/Blueprint/Enemy/DT_Ghost.DT_Ghost" (`|GetArrayItem` _outrownames `Row Index`))
    (:`then`
      (bind (_movespeed _hitcount _bhasbodyattack _bhasspecialattack _point _fireattackduration) (break `/Game/Blueprint/Enemy/GhostStatus` _returnvalue))
      (set `self.Init Move Speed` _movespeed)
      (set `self.HitCount` _hitcount)
      (set `self.bHasBodyAttack` _bhasbodyattack)
      (set `self.bHasSpecialAttack` _bhasspecialattack)
      (set `self.ScorePoint` _point)
      (set `self.Delay Time` _fireattackduration))))

(fn `UserConstructionScript`
  (`parent.UserConstructionScript`)
  (`self.Data Setup` (`self.Row Index`)))
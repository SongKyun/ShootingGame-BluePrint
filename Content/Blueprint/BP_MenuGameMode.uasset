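; Menu game mode that shows the home UI with a mouse cursor and runs a camera carousel over the level's tanks.
; BeginPlay finds the level's CameraActor, stores its start location and collects all BP_Player_Tank1 actors.
; SetFocusIndex cycles the focused tank with wraparound.
; StartMovement uses the Animator timeline to lerp the camera to that tank plus a fixed offset, then saves it as the next start.
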(event `self.ReceiveBeginPlay`
  (bind _returnvalue (`GameplayStatics.GetPlayerController` 0))
  (bind _returnvalue_2 (`|CreateWidget` "/Game/UI/WBP_HomeUI.WBP_HomeUI_C" _returnvalue))
  (`UserWidget.AddToViewport` _returnvalue_2 0)
  (set `PlayerController.bShowMouseCursor` true _returnvalue)
  (`WidgetBlueprintLibrary.SetInputMode_UIOnlyEx` _returnvalue _returnvalue_2)
  ;[1 1 1] 시작 시, 시작 위치를 카메라 위치로 초기화
  (`self.Find Camera`)
  (bind _cameraactor (`self.CameraActor`)
    (:`then`
      (set `self.StartPosition` (`self.K2_GetActorLocation` _cameraactor))
      ;[1 1 1] 탱크들을 찾아서 (Array)변수에 할당
      (bind _outactors (`GameplayStatics.GetAllActorsOfClass` "/Game/Blueprint/TankPlayer/BP_Player_Tank1.BP_Player_Tank1_C"))
      (set `self.Tanks` _outactors))
    (:`else`)))

(event `StartMovement`
  (bind _cameraactor (`self.CameraActor`))
  ;[1 1 1] Lerp StartMovement
  (`self.UpdateTargetLocation`)
  (bind (_direction _newtrack_0) (`Timeline|Animator` :!label _label)
    (:`Update`
      (`self.K2_SetActorLocation` _cameraactor (`KismetMathLibrary.VLerp` (`self.StartPosition`) (`self.TargetPosition`) _newtrack_0) false false))
    (:`Finished`
      (`self.K2_SetActorLocation` _cameraactor (`self.TargetPosition`) false false)
      (set `self.StartPosition` (`self.TargetPosition`))
      (goto _label :!via `SetNewTime`))))

(fn `Find Camera`
  (bind _returnvalue (`GameplayStatics.GetActorOfClass` "/Script/Engine.CameraActor"))
  (`/Engine/EditorBlueprintResources/StandardMacros.IsValid` _returnvalue
    (:`Is Valid`
      (set `self.CameraActor` _returnvalue))
    (:`Is Not Valid`
      (`KismetSystemLibrary.LogString` "Can't Find Camera"))))

(fn `SetFocusIndex`
  (params (Increase :type Boolean))
  (bind _currentfocusindex (`self.CurrentFocusIndex`))
  ;[1 1 1] Index 업데이트
  (if Increase
    (bind _result (`/Engine/EditorBlueprintResources/StandardMacros.IncrementInt` _currentfocusindex)
      (:`  `
        (if (>= _result (`KismetArrayLibrary.Array_Length` (`self.Tanks`)))
          (set `self.CurrentFocusIndex` 0))))
    (else
      (bind _result_2 (`/Engine/EditorBlueprintResources/StandardMacros.DecrementInt` _currentfocusindex)
        (:`  `
          (if (< _result_2 0)
            (set `self.CurrentFocusIndex` (- (`KismetArrayLibrary.Array_Length` (`self.Tanks`)) 1))))))))

(fn `UpdateTargetLocation`
  (set `self.TargetPosition` (+ (`self.K2_GetActorLocation` (`|GetArrayItem` (`self.Tanks`) (`self.CurrentFocusIndex`))) (260.0 0.0 130.0))))

(fn `UserConstructionScript`)